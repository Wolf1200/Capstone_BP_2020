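; BP_Capstone_2020Controller is a controller Blueprint that manages the inventory UI.
; It creates and caches a WB_Inventory widget on BeginPlay.
; The OpenInventory input recreates that widget if invalid, then adds it to the viewport and gives it keyboard focus.
; A ReloadInventory event tells the cached widget to load its inventory items again.
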(event EventBeginPlay
  (bind _returnvalue (UserInterface|CreateWidget "/Game/UI/WB_Inventory.WB_Inventory_C"))
  (Variables|Default|SetInventory%20Widget _returnvalue))

(event EventTick
  (params (DeltaSeconds :type Float%20%28single-precision%29)))

(event EventReloadInventory
  (bind _inventory_widget (Variables|Default|GetInventory%20Widget))
  (Utilities|IsValid _inventory_widget
    (:Is%20Valid
      (Default|LoadInventoryItems _inventory_widget))))

(event Input|ActionEvents|InputActionOpenInventory
  (params (Key :type Key%20Structure :default "None"))
  (:Pressed
    (Utilities|IsValid (Variables|Default|GetInventory%20Widget)
      (:Is%20Valid
        _)
      (:Is%20Not%20Valid
        (bind _returnvalue (UserInterface|CreateWidget "/Game/UI/WB_Inventory.WB_Inventory_C" (Game|GetPlayerController 0)))
        (bind _output_get (Variables|Default|SetInventory%20Widget _returnvalue))))
    (UserInterface|Viewport|AddtoViewport (Variables|Default|GetInventory%20Widget) 0)
    (Widget|SetKeyboardFocus _output_get)))

(fn ConstructionScript)